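; Projectile actor for a shooting game that destroys whatever it hits and awards a point.
; It destroys itself two seconds after BeginPlay if nothing is hit first.
; On Hit it spawns an explosion emitter, waits a zero-length delay, then destroys itself and the other actor without filtering by type.
; It then increments Score on the ShootingGameInstance.
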(event `self.ReceiveBeginPlay`
  (`KismetSystemLibrary.Delay` 2.0)
  (`self.K2_DestroyActor`))

(event `self.ReceiveHit`
  (params (MyComp :type "PrimitiveComponent Object Reference") (Other :type "Actor Object Reference") (OtherComp :type "PrimitiveComponent Object Reference") (bSelfMoved :type Boolean) (HitLocation :type "Vector Structure") (HitNormal :type "Vector Structure") (NormalImpulse :type "Vector Structure") (Hit :type "HitResult Structure (by ref)"))
  (`GameplayStatics.SpawnEmitterAtLocation` "/Game/StarterContent/Particles/P_Explosion.P_Explosion" HitLocation)
  (`KismetSystemLibrary.Delay` 0.0)
  (`self.K2_DestroyActor`)
  (`self.K2_DestroyActor` Other)
  (bind _asshooting_game_instance (cast `/Game/Blueprints/ShootingGameInstance` (`GameplayStatics.GetGameInstance`)))
  (set `/Game/Blueprints/ShootingGameInstance.Score` (+ (`/Game/Blueprints/ShootingGameInstance.Score` _asshooting_game_instance) 1) _asshooting_game_instance))

(fn `UserConstructionScript`)