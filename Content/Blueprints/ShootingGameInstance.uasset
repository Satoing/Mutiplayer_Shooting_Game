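; ShootingGameInstance is a game instance Blueprint that spawns the shooting game's UI screens.
; Four custom events each create a widget for the first player controller and add it to the viewport: opening, runtime, win ending and a second ending (EndUI_FEAT).
; It keeps no references to the created widgets and never removes them, and nothing in this graph calls the events.
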(event `CreateOpenUI`
  (bind _returnvalue (`|CreateWidget` "/Game/UI/Open/OpenUI.OpenUI_C" (`GameplayStatics.GetPlayerController` 0)))
  (`UserWidget.AddToViewport` _returnvalue 0))

(event `CreateRuntimeUI`
  (bind _returnvalue (`|CreateWidget` "/Game/UI/Runtime/RuntimeUI.RuntimeUI_C" (`GameplayStatics.GetPlayerController` 0)))
  (`UserWidget.AddToViewport` _returnvalue 0))

(event `CreateEndUI_1`
  (bind _returnvalue (`|CreateWidget` "/Game/UI/End/EndUI_WIN.EndUI_WIN_C" (`GameplayStatics.GetPlayerController` 0)))
  (`UserWidget.AddToViewport` _returnvalue 0))

(event `CreateEndUI_2`
  (bind _returnvalue (`|CreateWidget` "/Game/UI/End/EndUI_FEAT.EndUI_FEAT_C" (`GameplayStatics.GetPlayerController` 0)))
  (`UserWidget.AddToViewport` _returnvalue 0))